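; Spider actor Blueprint that walks a Spider component back and forth on an endless loop from BeginPlay.
; Timeline_3 adds a lerped step to relative X every update; the Rot timeline turns yaw by fixed per-update increments, triggered mid-loop and on finish.
; Stress-change tracking from the BP_SerialCom serial actor feeds an unfinished walkSpider event, which is never called here and doesn't yet affect movement.
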(event Custom|SpiderRot
  (bind _spider (Variables|Default|GetSpider))
  (bind _relativerotation (Variables|/Script/Engine.SceneComponent|GetRelativeRotation _spider))
  (bind (_roll _pitch _yaw) (Math|Rotator|BreakRotator _relativerotation))
  ;[1 1 1] When called by SpiderRot, the spider will rotate 90 degrees before moving in the other direction
  (Timeline|Rot PlayFromStart
    (:Update
      (Transformation|SetRelativeRotation _spider (Math|Rotator|MakeRotator _roll _pitch (+ -1.5 _yaw)) false false))))

(event Custom|walkSpider
  ;[1 1 1] WIP Section for better Spider movement
  (CallFunction|ReadStressValue)
  (if (== (Variables|Default|GetstressChange) 0)
    _))

(event Custom|readStressValue
  ;[0.224 0.224 0.224] This  section allows the spider to read in the stress from the Serial object and tracks the stress value and whether it increased, decreased, or stayed the same
  (bind _returnvalue (Actor|GetActorOfClass "/Game/BP_SerialCom_v4_UE510.BP_SerialCom_v4_UE510_C"))
  (if (> (Variables|/Game/BP_SerialCom_v4_UE510.BP_SerialCom_v4_UE510_C|GetstressVal _returnvalue) (Variables|Default|GetstressLVL))
    (Variables|Default|SetstressChange 1)
    (elif (> (Variables|Default|GetstressLVL) (Variables|/Game/BP_SerialCom_v4_UE510.BP_SerialCom_v4_UE510_C|GetstressVal _returnvalue))
      (Variables|Default|SetstressChange -1)
      (else
        (Variables|Default|SetstressChange 0))))
  (Variables|Default|SetstressLVL (Variables|/Game/BP_SerialCom_v4_UE510.BP_SerialCom_v4_UE510_C|GetstressVal _returnvalue)))

(event EventBeginPlay
  (bind _spider (Variables|Default|GetSpider))
  (bind _relativelocation (Variables|/Script/Engine.SceneComponent|GetRelativeLocation _spider))
  (bind (_x _y _z) (Math|Vector|BreakVector _relativelocation))
  ;[1 1 1] Spider will
  (Utilities|FlowControl|Sequence :!label _label
    (:then_0
      ;[1 1 1] Spider will move from A_0 = -2 to B_0 = 2 on a loop
      (bind _newtrack_0 (Timeline|Timeline_3 PlayFromStart)
        (:Update
          (Transformation|SetRelativeLocation _spider (Math|Vector|MakeVector (+ _x (Math|Float|Lerp (Variables|Default|GetA_0) (Variables|Default|GetB_0) _newtrack_0)) _y _z) false false))
        (:Finished
          (CallFunction|SpiderRot)
          (Utilities|FlowControl|Delay 1.0)
          (goto _label))))
    (:then_1
      (Utilities|FlowControl|Delay 1.0)
      (CallFunction|SpiderRot))))

(fn ConstructionScript)